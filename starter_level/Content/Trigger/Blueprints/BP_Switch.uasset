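; BP_Switch is an interactable light switch that toggles a SpotLight and reports device usage to the player character.
; Its Box overlap sends interact-area enter and exit messages to the overlapping actor.
; DoMyInteraction flip-flops off first, then on, adjusting the player's OpenDevices count.
; Only switching on adds Watt to WattUsed; switching off never subtracts it, and AddOrMinusWatt's addition is unconnected.
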(event `self.ReceiveBeginPlay`
  (bind _asbp_trigger_trigger_third_person_character (cast `/Game/Trigger/Blueprints/BP_Trigger_TriggerThirdPersonCharacter` (`GameplayStatics.GetPlayerCharacter` 0)))
  (set `self.Ref` _asbp_trigger_trigger_third_person_character))

(event `self.Box.OnComponentBeginOverlap`
  (params (OverlappedComponent :type "PrimitiveComponent Object Reference") (OtherActor :type "Actor Object Reference") (OtherComp :type "PrimitiveComponent Object Reference") (OtherBodyIndex :type Integer) (bFromSweep :type Boolean) (SweepResult :type "HitResult Structure (by ref)"))
  (message `/Game/Trigger/Blueprints/BPI_Active.InteractAreaEntered` OtherActor self))

(event `self.Box.OnComponentEndOverlap`
  (params (OverlappedComponent :type "PrimitiveComponent Object Reference") (OtherActor :type "Actor Object Reference") (OtherComp :type "PrimitiveComponent Object Reference") (OtherBodyIndex :type Integer))
  (message `/Game/Trigger/Blueprints/BPI_Active.InteractAreaExited` OtherActor null))

(event `/Game/Trigger/Blueprints/BPI_Active.Do My Interaction`
  (bind _spotlight (`self.SpotLight`))
  ;[1 1 1] Set Visibility
  (`/Engine/EditorBlueprintResources/StandardMacros.FlipFlop`
    (:`A`
      (bind _output_get (set `self.LightChecker` false))
      (`SceneComponent.SetVisibility` _spotlight _output_get false)
      (bind _asbp_trigger_trigger_third_person_character (cast `/Game/Trigger/Blueprints/BP_Trigger_TriggerThirdPersonCharacter` (`GameplayStatics.GetPlayerCharacter` 0)))
      (set `/Game/Trigger/Blueprints/BP_Trigger_TriggerThirdPersonCharacter.OpenDevices` (- (`/Game/Trigger/Blueprints/BP_Trigger_TriggerThirdPersonCharacter.OpenDevices` _asbp_trigger_trigger_third_person_character) 1) _asbp_trigger_trigger_third_person_character))
    (:`B`
      (bind _output_get_2 (set `self.LightChecker` true))
      (`SceneComponent.SetVisibility` _spotlight _output_get_2 false)
      (bind _asbp_trigger_trigger_third_person_character_2 (cast `/Game/Trigger/Blueprints/BP_Trigger_TriggerThirdPersonCharacter` (`GameplayStatics.GetPlayerCharacter` 0)))
      (set `/Game/Trigger/Blueprints/BP_Trigger_TriggerThirdPersonCharacter.WattUsed` (+ (`/Game/Trigger/Blueprints/BP_Trigger_TriggerThirdPersonCharacter.WattUsed` _asbp_trigger_trigger_third_person_character_2) (`self.Watt`)) _asbp_trigger_trigger_third_person_character_2)
      (set `/Game/Trigger/Blueprints/BP_Trigger_TriggerThirdPersonCharacter.OpenDevices` (+ (`/Game/Trigger/Blueprints/BP_Trigger_TriggerThirdPersonCharacter.OpenDevices` _asbp_trigger_trigger_third_person_character_2) 1) _asbp_trigger_trigger_third_person_character_2))))

(fn `Add or Minus Watt`
  (bind _asbp_trigger_trigger_third_person_character (cast `/Game/Trigger/Blueprints/BP_Trigger_TriggerThirdPersonCharacter` (`GameplayStatics.GetPlayerCharacter` 0))))

(fn `UserConstructionScript`)