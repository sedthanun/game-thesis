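; FallvolumeBP is a kill volume that restarts the current level when the player character enters it.
; Its construction script sizes the Overlap box from a BoxExtent variable, so each placed volume can set its own bounds.
; On overlap with the third-person character, it plays a 2D sound, prints a death message and shows a FadeToBlack widget.
; After a short delay, it reopens the current level by name.
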(event `self.Overlap.OnComponentBeginOverlap`
  (params (OverlappedComponent :type "PrimitiveComponent Object Reference") (OtherActor :type "Actor Object Reference") (OtherComp :type "PrimitiveComponent Object Reference") (OtherBodyIndex :type Integer) (bFromSweep :type Boolean) (SweepResult :type "HitResult Structure (by ref)"))
  (cast `/Game/Trigger/Blueprints/BP_Trigger_TriggerThirdPersonCharacter` OtherActor)
  (`GameplayStatics.SpawnSound2D` "/Game/StarterContent/Audio/SEEN1.SEEN1" 1.0 1.0 0.0 null)
  (`KismetSystemLibrary.PrintString` "You Died!")
  (bind _returnvalue (`|CreateWidget` "/Game/Checkpoint/FadetoBlack.FadeToBlack_C"))
  (`/Game/Checkpoint/FadetoBlack.FadeToBlack` _returnvalue)
  (`UserWidget.AddToViewport` _returnvalue 0)
  (`KismetSystemLibrary.Delay` 3.0)
  (bind _returnvalue_2 (`GameplayStatics.GetCurrentLevelName` true))
  (`GameplayStatics.OpenLevel` (`KismetStringLibrary.Conv_StringToName` _returnvalue_2)))

(fn `UserConstructionScript`
  (`BoxComponent.SetBoxExtent` (`self.Overlap`) (`self.Box Extent`) true))