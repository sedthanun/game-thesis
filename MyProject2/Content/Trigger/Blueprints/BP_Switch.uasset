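; BP_Switch is an interactable switch that toggles a SpotLight and adds its Watt value to the player character's WattUsed.
; Box overlaps send interact-area entered and exited messages to the overlapping actor.
; DoMyInteraction uses a FlipFlop with only the A branch wired, so every other interaction toggles the light and adds wattage, with no subtraction.
; AddOrMinusWatt only casts the player, leaving its addition disconnected.
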(event `self.ReceiveBeginPlay`
  (bind _asbp_trigger_third_person_character (cast `/Game/Trigger/Blueprints/BP_Trigger_ThirdPersonCharacter` (`GameplayStatics.GetPlayerCharacter` 0)))
  (set `self.Ref` _asbp_trigger_third_person_character))

(event `self.Box.OnComponentBeginOverlap`
  (params (OverlappedComponent :type "PrimitiveComponent Object Reference") (OtherActor :type "Actor Object Reference") (OtherComp :type "PrimitiveComponent Object Reference") (OtherBodyIndex :type Integer) (bFromSweep :type Boolean) (SweepResult :type "HitResult Structure (by ref)"))
  (message `/Game/Trigger/Blueprints/BPI_Active.InteractAreaEntered` OtherActor self))

(event `self.Box.OnComponentEndOverlap`
  (params (OverlappedComponent :type "PrimitiveComponent Object Reference") (OtherActor :type "Actor Object Reference") (OtherComp :type "PrimitiveComponent Object Reference") (OtherBodyIndex :type Integer))
  (message `/Game/Trigger/Blueprints/BPI_Active.InteractAreaExited` OtherActor null))

(event `/Game/Trigger/Blueprints/BPI_Active.Do My Interaction`
  (`/Engine/EditorBlueprintResources/StandardMacros.FlipFlop`
    (:`A`
      (bind _asbp_trigger_third_person_character (cast `/Game/Trigger/Blueprints/BP_Trigger_ThirdPersonCharacter` (`GameplayStatics.GetPlayerCharacter` 0)))
      (set `/Game/Trigger/Blueprints/BP_Trigger_ThirdPersonCharacter.WattUsed` (+ (`/Game/Trigger/Blueprints/BP_Trigger_ThirdPersonCharacter.WattUsed` _asbp_trigger_third_person_character) (`self.Watt`)) _asbp_trigger_third_person_character)
      (`SceneComponent.ToggleVisibility` (`self.SpotLight`) false))))

(fn `Add or Minus Watt`
  (bind _asbp_trigger_third_person_character (cast `/Game/Trigger/Blueprints/BP_Trigger_ThirdPersonCharacter` (`GameplayStatics.GetPlayerCharacter` 0))))

(fn `UserConstructionScript`)